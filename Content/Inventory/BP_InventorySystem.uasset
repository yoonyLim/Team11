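; Slot-based inventory with item stacking, quality, carried weight, and helmet, chest armor and weapon equipment slots.
; BeginPlay creates empty GUID-tagged slots; adding fills matching stacks then empty slots using InventoryItems DataTable stack limits, while removal drains the last stacks first.
; Right-clicking equips an item by type, returning any replaced item through AddItem, which also handles unequipping.
; ReloadData recalculates weight including equipped gear and broadcasts OnInventoryUpdated.
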(event `self.ReceiveBeginPlay`
  (`self.CreateInventory`))

(event `OnRightMouseButtonOnItem`
  (params (Slot :type "/Game/Inventory/S_InventorySlot Structure") (Item :type "/Game/Inventory/S_InventoryItem Structure"))
  (switch `/Game/Inventory/E_EquipmentType` (`.EquipmentType_22_312868C14BEB5FB6A17FF2BE529BED1D` (break `/Game/Inventory/S_InventoryItem` Item))
    (:`NewEnumerator0`
      (`self.EquipArmor` Slot :!label _label))
    (:`NewEnumerator1`
      (goto _label))
    (:`NewEnumerator2`
      (`self.EquipWeapon` Slot))))

(fn `AddItem`
  (params (ID :type String) (Amount :type Integer) (Quality :type "Float (double-precision)" :default -1.0))
  (locals (Local_AmountLeft :type Integer))
  (set `local.Local_AmountLeft` Amount)
  (bind (_collectedamount _outslots) (`self.FindSlotsToStore` ID Amount (`self.Find Items` ID)))
  (for _array_element _outslots
    (bind _returnvalue (`|GetDataTableRow` "/Game/Inventory/InventoryItems.InventoryItems" (`KismetStringLibrary.Conv_StringToName` (`local.ID`)))
      (:`then`
        (bind (_uuid _item _amount _id _itemquality) (break `/Game/Inventory/S_InventorySlot` _array_element))
        (bind _returnvalue_2 (`KismetMathLibrary.Min` (- (`.MaxStackSize_11_A8CD777244882EC402D655B1C4426C8F` (break `/Game/Inventory/S_InventoryItem` _returnvalue)) _amount) (`local.Local_AmountLeft`)))
        (`KismetArrayLibrary.Array_Set` (`self.Inventory`) (`KismetArrayLibrary.Array_Find` (`self.Inventory`) _array_element) (make `/Game/Inventory/S_InventorySlot` _uuid (make `DataTableRowHandle` "/Game/Inventory/InventoryItems.InventoryItems" (`KismetStringLibrary.Conv_StringToName` (`local.ID`))) (+ _amount _returnvalue_2) (`local.ID`) (`KismetMathLibrary.SelectFloat` (`local.Quality`) _itemquality (!= (`local.Quality`) -1.0))))
        (set `local.Local_AmountLeft` (- (`local.Local_AmountLeft`) _returnvalue_2)))))
  (`self.ReloadData`))

(fn `CalculateWeight`
  (returns (Weight :type "Float (double-precision)"))
  (locals (Local_AllItems :type "Array of /Game/Inventory/S_InventorySlot Structure") (Local_Weight :type "Float (double-precision)"))
  (set `local.Local_AllItems` (`self.Inventory`))
  (for _array_element (`|MakeArray` (`self.HelmetSlot`) (`self.ChestArmorSlot`) (`self.WeaponSlot`))
    (`KismetArrayLibrary.Array_Add` (`local.Local_AllItems`) _array_element))
  (for _array_element_2 (`local.Local_AllItems`)
    (bind (_uuid _item _amount) (break `/Game/Inventory/S_InventorySlot` _array_element_2))
    (bind (_datatable _rowname) (break `DataTableRowHandle` _item))
    (`/Engine/EditorBlueprintResources/StandardMacros.IsValid` _datatable
      (:`Is Valid`
        (bind _returnvalue (`|GetDataTableRow` _datatable _rowname)
          (:`then`
            (set `local.Local_Weight` (+ (`local.Local_Weight`) (* (`.Weight_14_6266DEF9497CFBF2809EF29392E15C7A` (break `/Game/Inventory/S_InventoryItem` _returnvalue)) _amount))))))))
  (return (`local.Local_Weight`)))

(fn `CreateInventory`
  (for _ (range 1 (+ (`self.MaxSlotsCount`) 1))
    (`KismetArrayLibrary.Array_Add` (`self.Inventory`) (make `/Game/Inventory/S_InventorySlot` (`KismetGuidLibrary.Conv_GuidToString` (`KismetGuidLibrary.NewGuid`))))))

(fn `DeequipItem`
  (params (Slot :type "/Game/Inventory/S_InventorySlot Structure"))
  (locals (DeequipID :type String))
  (bind ((`UUID_2_3ACFCEA5488A4477040A5EA05753F0F1` _uuid)) (break `/Game/Inventory/S_InventorySlot` Slot))
  (bind ((`Amount_8_953AFCFF43CBE5320DF0EEB65F8FD17B` _amount) (`ID_11_C98737B9456B10E95A90828B6E0641EA` _id) (`ItemQuality_14_3F3290CA4BC16F09D7841E9BE7571280` _itemquality)) (break `/Game/Inventory/S_InventorySlot` (`local.Slot`)))
  (set `local.DeequipID` _uuid)
  (if (`KismetStringLibrary.EqualEqual_StrStr` _uuid (`.UUID_2_3ACFCEA5488A4477040A5EA05753F0F1` (break `/Game/Inventory/S_InventorySlot` (`self.HelmetSlot`))))
    (set `self.HelmetSlot` (struct))
    (`self.AddItem` _id _amount _itemquality :!label _label)
    (elif (`KismetStringLibrary.EqualEqual_StrStr` (`local.DeequipID`) (`.UUID_2_3ACFCEA5488A4477040A5EA05753F0F1` (break `/Game/Inventory/S_InventorySlot` (`self.ChestArmorSlot`))))
      (set `self.ChestArmorSlot` (struct))
      (goto _label)
      (elif (`KismetStringLibrary.EqualEqual_StrStr` (`local.DeequipID`) (`.UUID_2_3ACFCEA5488A4477040A5EA05753F0F1` (break `/Game/Inventory/S_InventorySlot` (`self.WeaponSlot`))))
        (set `self.WeaponSlot` (struct))
        (goto _label)))))

(fn `EquipArmor`
  (params (Slot :type "/Game/Inventory/S_InventorySlot Structure"))
  (locals (PreviousArmorSlot :type "/Game/Inventory/S_InventorySlot Structure"))
  (bind _slot (`local.Slot`))
  (bind ((`UUID_2_3ACFCEA5488A4477040A5EA05753F0F1` _uuid) (`ItemQuality_14_3F3290CA4BC16F09D7841E9BE7571280` _itemquality)) (break `/Game/Inventory/S_InventorySlot` (`local.Slot`)))
  (bind (_datatable _rowname) (break `DataTableRowHandle` (`.Item_5_372C6A40474FEEC5F6052185298FB7DC` (break `/Game/Inventory/S_InventorySlot` Slot))))
  (bind _returnvalue (`|GetDataTableRow` _datatable _rowname)
    (:`then`
      (`|ExecutionSequence`
        (:`then_0`
          (bind ((`EquipmentType_22_312868C14BEB5FB6A17FF2BE529BED1D` _equipmenttype)) (break `/Game/Inventory/S_InventoryItem` _returnvalue))
          (bind _returnvalue_2 (select `/Game/Inventory/E_EquipmentType` _equipmenttype :`NewEnumerator0` (`self.HelmetSlot`) :`NewEnumerator1` (`self.ChestArmorSlot`)))
          (if (== (`.Amount_8_953AFCFF43CBE5320DF0EEB65F8FD17B` (break `/Game/Inventory/S_InventorySlot` _returnvalue_2)) 0)
            (switch `/Game/Inventory/E_EquipmentType` _equipmenttype :!label _label
              (:`NewEnumerator0`
                (set `self.HelmetSlot` _slot))
              (:`NewEnumerator1`
                (set `self.ChestArmorSlot` _slot)))
            (`KismetArrayLibrary.Array_Set` (`self.Inventory`) (`KismetArrayLibrary.Array_Find` (`self.Inventory`) (`local.Slot`)) (make `/Game/Inventory/S_InventorySlot` :`UUID` _uuid :`ItemQuality` _itemquality))
            (else
              (bind _output_get (set `local.PreviousArmorSlot` _returnvalue_2))
              (`|ExecutionSequence`
                (:`then_0`
                  (goto _label))
                (:`then_1`
                  (bind ((`Amount_8_953AFCFF43CBE5320DF0EEB65F8FD17B` _amount) (`ID_11_C98737B9456B10E95A90828B6E0641EA` _id) (`ItemQuality_14_3F3290CA4BC16F09D7841E9BE7571280` _itemquality_2)) (break `/Game/Inventory/S_InventorySlot` _output_get))
                  (`self.AddItem` _id _amount _itemquality_2))))))
        (:`then_1`
          (`self.ReloadData`))))))

(fn `EquipWeapon`
  (params (Slot :type "/Game/Inventory/S_InventorySlot Structure"))
  (locals (PreviousWeaponSlot :type "/Game/Inventory/S_InventorySlot Structure"))
  (bind ((`UUID_2_3ACFCEA5488A4477040A5EA05753F0F1` _uuid) (`ItemQuality_14_3F3290CA4BC16F09D7841E9BE7571280` _itemquality)) (break `/Game/Inventory/S_InventorySlot` (`local.Slot`)))
  (bind ((`Amount_8_953AFCFF43CBE5320DF0EEB65F8FD17B` _amount) (`ID_11_C98737B9456B10E95A90828B6E0641EA` _id) (`ItemQuality_14_3F3290CA4BC16F09D7841E9BE7571280` _itemquality_2)) (break `/Game/Inventory/S_InventorySlot` (`local.PreviousWeaponSlot`)))
  (`|ExecutionSequence`
    (:`then_0`
      (if (== (`.Amount_8_953AFCFF43CBE5320DF0EEB65F8FD17B` (break `/Game/Inventory/S_InventorySlot` (`self.WeaponSlot`))) 0)
        (set `self.WeaponSlot` (`local.Slot`) :!label _label)
        (`KismetArrayLibrary.Array_Set` (`self.Inventory`) (`KismetArrayLibrary.Array_Find` (`self.Inventory`) (`local.Slot`)) (make `/Game/Inventory/S_InventorySlot` :`UUID` _uuid :`ItemQuality` _itemquality))
        (else
          (set `local.PreviousWeaponSlot` (`self.WeaponSlot`))
          (`|ExecutionSequence`
            (:`then_0`
              (goto _label))
            (:`then_1`
              (`self.AddItem` _id _amount _itemquality_2))))))
    (:`then_1`
      (`self.ReloadData`))))

(fn `Find Items`
  (params (ID :type String))
  (returns (Slots :type "Array of /Game/Inventory/S_InventorySlot Structure"))
  (locals (Local_Slots :type "Array of /Game/Inventory/S_InventorySlot Structure"))
  (for _array_element (`self.Inventory`)
    (if (`KismetStringLibrary.EqualEqual_StrStr` (`.ID_11_C98737B9456B10E95A90828B6E0641EA` (break `/Game/Inventory/S_InventorySlot` _array_element)) (`local.ID`))
      (`KismetArrayLibrary.Array_Add` (`local.Local_Slots`) _array_element)))
  (return (`local.Local_Slots`)))

(fn `FindEmptySlots`
  (returns (Slots :type "Array of /Game/Inventory/S_InventorySlot Structure"))
  (locals (Local_Slots :type "Array of /Game/Inventory/S_InventorySlot Structure"))
  (for _array_element (`self.Inventory`)
    (if (== (`.Amount_8_953AFCFF43CBE5320DF0EEB65F8FD17B` (break `/Game/Inventory/S_InventorySlot` _array_element)) 0)
      (`KismetArrayLibrary.Array_Add` (`local.Local_Slots`) _array_element)))
  (return (`local.Local_Slots`)))

(fn `FindSlotsToStore`
  (params (ID :type String) (Amount :type Integer) (Slots :type "Array of /Game/Inventory/S_InventorySlot Structure"))
  (returns (CollectedAmount :type Integer) (OutSlots :type "Array of /Game/Inventory/S_InventorySlot Structure"))
  (locals (StorableAmountLeft :type Integer) (Local_Slots :type "Array of /Game/Inventory/S_InventorySlot Structure"))
  (set `local.StorableAmountLeft` Amount)
  (for _array_element Slots
    (bind (_uuid _item _amount) (break `/Game/Inventory/S_InventorySlot` _array_element))
    (bind (_datatable _rowname) (break `DataTableRowHandle` _item))
    (bind _returnvalue (`|GetDataTableRow` _datatable _rowname)
      (:`then`
        (bind (_id _name _thumbnail _maxstacksize) (break `/Game/Inventory/S_InventoryItem` _returnvalue))
        (if (!= _maxstacksize _amount)
          (`KismetArrayLibrary.Array_Add` (`local.Local_Slots`) _array_element)
          (bind _output_get (set `local.StorableAmountLeft` (`KismetMathLibrary.Clamp` (- (`local.StorableAmountLeft`) (- _maxstacksize _amount (`local.Amount`))) 0 (`local.Amount`))))
          (if (== _output_get 0)
            (break))))))
  (`|ExecutionSequence`
    (:`then_0`
      (if (not (== (`local.StorableAmountLeft`) 0))
        (bind _returnvalue_2 (`|GetDataTableRow` "/Game/Inventory/InventoryItems.InventoryItems" (`KismetStringLibrary.Conv_StringToName` (`local.ID`)))
          (:`then`
            (for _array_element_2 (`self.FindEmptySlots`)
              (set `local.StorableAmountLeft` (`KismetMathLibrary.Clamp` (- (`local.StorableAmountLeft`) (`.MaxStackSize_11_A8CD777244882EC402D655B1C4426C8F` (break `/Game/Inventory/S_InventoryItem` _returnvalue_2))) 0 (`local.Amount`)))
              (`KismetArrayLibrary.Array_Add` (`local.Local_Slots`) _array_element_2)
              (if (== (`local.StorableAmountLeft`) 0)
                (break)))))))
    (:`then_1`
      (return (- (`local.Amount`) (`local.StorableAmountLeft`)) (`local.Local_Slots`)))))

(fn `ReloadData`
  (bind _weight (`self.CalculateWeight`))
  (set `self.CurrentWeight` _weight)
  (`self.OnInventoryUpdated`))

(fn `RemoveItem`
  (params (ID :type String) (Amount :type Integer))
  (locals (Local_RemoveLeft :type Integer) (Local_Slots :type "Array of /Game/Inventory/S_InventorySlot Structure") (Local_Inventory :type "Array of /Game/Inventory/S_InventorySlot Structure"))
  (bind _output_get (set `local.Local_Inventory` (`self.Inventory`)))
  (`KismetArrayLibrary.Array_Reverse` _output_get)
  (set `local.Local_RemoveLeft` Amount)
  (bind _output_get_2 (set `local.Local_Slots` (`self.Find Items` ID)))
  (`KismetArrayLibrary.Array_Reverse` _output_get_2)
  (for _array_element (`local.Local_Slots`)
    (bind (_uuid _item _amount _id _itemquality) (break `/Game/Inventory/S_InventorySlot` _array_element))
    (bind _returnvalue (`KismetMathLibrary.Min` (`local.Local_RemoveLeft`) _amount))
    (bind _returnvalue_2 (- _amount _returnvalue))
    (bind _returnvalue_3 (== _returnvalue_2 0))
    (`KismetArrayLibrary.Array_Set` (`self.Inventory`) (- (- (`KismetArrayLibrary.Array_Length` (`local.Local_Inventory`)) 1) (`KismetArrayLibrary.Array_Find` (`local.Local_Inventory`) _array_element)) (make `/Game/Inventory/S_InventorySlot` _uuid (select `bool` _returnvalue_3 :`false` _item) _returnvalue_2 (select `bool` _returnvalue_3 :`false` _id) _itemquality))
    (bind _output_get_3 (set `local.Local_RemoveLeft` (- (`local.Local_RemoveLeft`) _returnvalue)))
    (if (== _output_get_3 0)
      (break)))
  (`self.ReloadData`))