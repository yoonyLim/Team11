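; Component that manages which UI widgets, the main HUD and inventory, are shown and when the mouse cursor appears.
; ShowWidget and HideWidget track open widget types in a set, lazily creating W_MainHUD with the owner's BP_InventorySystem and toggling the inventory through that HUD.
; Each change intersects the open set with CursorWidgets to switch between game-and-UI input with cursor and game-only input.
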(fn `HideWidget`
  (params (WidgetType :type "/Game/Inventory/WidgetsManager/E_WidgetType Enum" :default "NewEnumerator0"))
  (if (`BlueprintSetLibrary.Set_Contains` (`self.ShowWidgets`) WidgetType)
    (`|ExecutionSequence`
      (:`then_0`
        (switch `/Game/Inventory/WidgetsManager/E_WidgetType` (`local.WidgetType`)
          (:`NewEnumerator0`
            (`/Game/Inventory/UI/W_MainHUD.ShowInventory` (`self.MainHUDWidget`) false))
          (:`NewEnumerator1`
            (`Widget.RemoveFromParent` (`self.MainHUDWidget`)))))
      (:`then_1`
        (`BlueprintSetLibrary.Set_Remove` (`self.ShowWidgets`) (`local.WidgetType`))
        (`self.UpdateCursorVisibility`)))))

(fn `ShowWidget`
  (params (WidgetType :type "/Game/Inventory/WidgetsManager/E_WidgetType Enum" :default "NewEnumerator0"))
  (if (not (`BlueprintSetLibrary.Set_Contains` (`self.ShowWidgets`) WidgetType))
    (`|ExecutionSequence`
      (:`then_0`
        (switch `/Game/Inventory/WidgetsManager/E_WidgetType` (`local.WidgetType`)
          (:`NewEnumerator0`
            (`/Game/Inventory/UI/W_MainHUD.ShowInventory` (`self.MainHUDWidget`) true))
          (:`NewEnumerator1`
            (`/Engine/EditorBlueprintResources/StandardMacros.IsValid` (`self.MainHUDWidget`)
              (:`Is Valid`
                (`UserWidget.AddToViewport` (`self.MainHUDWidget`) 0))
              (:`Is Not Valid`
                (bind _returnvalue (`|CreateWidget` "/Game/Inventory/UI/W_MainHUD.W_MainHUD_C" null (`Actor.GetComponentByClass` (`self.GetOwner`) "/Game/Inventory/BP_InventorySystem.BP_InventorySystem_C")))
                (bind _output_get (set `self.MainHUDWidget` _returnvalue))
                (`UserWidget.AddToViewport` _output_get 0))))))
      (:`then_1`
        (`BlueprintSetLibrary.Set_Add` (`self.ShowWidgets`) (`local.WidgetType`))
        (`self.UpdateCursorVisibility`)))))

(fn `UpdateCursorVisibility`
  (bind _returnvalue (`GameplayStatics.GetPlayerController` 0))
  (bind _result (`BlueprintSetLibrary.Set_Intersection` (`self.ShowWidgets`) (`self.CursorWidgets`)))
  (if (`BlueprintSetLibrary.Set_IsNotEmpty` _result)
    (`WidgetBlueprintLibrary.SetInputMode_GameAndUIEx` _returnvalue null)
    (set `PlayerController.bShowMouseCursor` true _returnvalue)
    (else
      (`WidgetBlueprintLibrary.SetInputMode_GameOnly` _returnvalue)
      (set `PlayerController.bShowMouseCursor` false _returnvalue))))