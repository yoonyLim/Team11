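; BPC_ActiveQuest is a quest system component that shows the name of the active quest on screen.
; On BeginPlay it creates a WB_ActiveQuest widget, adds it to the viewport and keeps it hidden.
; The SetActiveQuest event copies the ActiveQuest name into the widget's text and makes the widget visible.
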(event `self.ReceiveBeginPlay`
  (bind _returnvalue (`|CreateWidget` "/Game/UI/Widgets/WB_ActiveQuest.WB_ActiveQuest_C"))
  (bind _output_get (set `self.ActiveQuestWidget` _returnvalue))
  (`UserWidget.AddToViewport` _output_get 0)
  (set `Widget.Visibility` "Hidden" _output_get))

(event `Set Active Quest`
  (bind _activequestwidget (`self.ActiveQuestWidget`))
  (bind _activequest_name (break `/Game/QuestSystem/F_QuestInfo` (`self.ActiveQuest`)))
  (set `TextBlock.Text` (`KismetTextLibrary.Conv_StringToText` _activequest_name) (`/Game/UI/Widgets/WB_ActiveQuest.ActiveQuestName` _activequestwidget))
  (set `Widget.Visibility` "Visible" _activequestwidget))