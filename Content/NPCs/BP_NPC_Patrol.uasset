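; Patrolling NPC Blueprint with a modular body that the player can interact with to step through lines of dialogue.
; Interacting halts the AI's brain logic and freezes both NPC and player movement, then creates or advances a WB_QuestDialogue widget through the Dialogues array.
; Running past the last line removes the widget, resets dialogue state and restores movement and AI logic.
; The construction script makes the body-part meshes follow the main Mesh via leader pose.
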(event `/Game/GameSystems/BPI_Interaction.InteractWith`
  (bind _dialoguewidget (`self.DialogueWidget`))
  (bind _charactermovement (`Character.CharacterMovement` (`GameplayStatics.GetPlayerCharacter` 0)))
  (bind _aicnpcbase (`self.AICNPCBase`)
    (:`then`
      (`BrainComponent.StopLogic` (`AIController.BrainComponent` _aicnpcbase) "")
      (`CharacterMovementComponent.DisableMovement` (`self.CharacterMovement`))
      (`CharacterMovementComponent.DisableMovement` _charactermovement)
      (if (`self.IsDialogueActive`)
        (set `TextBlock.Text` (`KismetTextLibrary.Conv_StringToText` (`|GetArrayItem` (`self.Dialogues`) (`self.DialoguesIndex`))) (`/Game/UI/Widgets/WB_QuestDialogue.DialogueText` _dialoguewidget))
        (bind _result (`/Engine/EditorBlueprintResources/StandardMacros.IncrementInt` (`self.DialoguesIndex`))
          (:`  `
            (if (< (`KismetArrayLibrary.Array_Length` (`self.Dialogues`)) _result)
              (`Widget.RemoveFromParent` _dialoguewidget)
              (set `self.DialoguesIndex` 0)
              (set `self.IsDialogueActive` false)
              (`CharacterMovementComponent.SetMovementMode` _charactermovement "MOVE_Walking" 0)
              (bind _aicnpcbase_2 (`self.AICNPCBase`)
                (:`then`
                  (`BrainComponent.RestartLogic` (`AIController.BrainComponent` _aicnpcbase_2))
                  (`CharacterMovementComponent.SetMovementMode` (`self.CharacterMovement`) "MOVE_Walking" 0))
                (:`else`)))))
        (else
          (bind _returnvalue (`|CreateWidget` "/Game/UI/Widgets/WB_QuestDialogue.WB_QuestDialogue_C"))
          (bind _output_get (set `self.DialogueWidget` _returnvalue))
          (set `TextBlock.Text` (`KismetTextLibrary.Conv_StringToText` (`|GetArrayItem` (`self.Dialogues`))) (`/Game/UI/Widgets/WB_QuestDialogue.DialogueText` _output_get))
          (`UserWidget.AddToViewport` _output_get 0)
          (set `self.IsDialogueActive` true)
          (`/Engine/EditorBlueprintResources/StandardMacros.IncrementInt` (`self.DialoguesIndex`)))))
    (:`else`)))

(fn `UserConstructionScript`
  (`SkinnedMeshComponent.SetLeaderPoseComponent` (`self.Legs`) (`self.Mesh`) false false)
  (`SkinnedMeshComponent.SetLeaderPoseComponent` (`self.Hands`) (`self.Mesh`) false false)
  (`SkinnedMeshComponent.SetLeaderPoseComponent` (`self.Head`) (`self.Mesh`) false false)
  (`SkinnedMeshComponent.SetLeaderPoseComponent` (`self.Feet`) (`self.Mesh`) false false)
  (`SkinnedMeshComponent.SetLeaderPoseComponent` (`self.Hat`) (`self.Mesh`) false false))