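; Base NPC character with a player-proximity interaction prompt, movement speed presets and hit reactions.
; The construction script makes separate leg, hand, head and foot meshes follow the main mesh's pose, and the trigger shows or hides the prompt widget.
; Hits play a directional montage, or an overlay material with a short timer and a world camera shake.
; Interact and close-widget events are empty; getters expose the patrol route and a zero ideal range.
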(event `self.ReceiveBeginPlay`
  (`SceneComponent.SetVisibility` (`self.WB_Interaction`) false false))

(event `self.InteractionTrigger.OnComponentBeginOverlap`
  (params (OverlappedComponent :type "PrimitiveComponent Object Reference") (OtherActor :type "Actor Object Reference") (OtherComp :type "PrimitiveComponent Object Reference") (OtherBodyIndex :type Integer) (bFromSweep :type Boolean) (SweepResult :type "HitResult Structure (by ref)"))
  (cast `/Game/Player/BluePrints/BP_Player` OtherActor)
  (`SceneComponent.SetVisibility` (`self.WB_Interaction`) true false))

(event `self.InteractionTrigger.OnComponentEndOverlap`
  (params (OverlappedComponent :type "PrimitiveComponent Object Reference") (OtherActor :type "Actor Object Reference") (OtherComp :type "PrimitiveComponent Object Reference") (OtherBodyIndex :type Integer))
  (cast `/Game/Player/BluePrints/BP_Player` OtherActor)
  (`SceneComponent.SetVisibility` (`self.WB_Interaction`) false false))

(event `/Game/GameSystems/BPI_Interaction.InteractWith`)

(event `CloseWidget`)

(event `/Game/Enemies/Interfaces/BPI_Enemy.SetMovementSpeed`
  (params (MovementSpeed :type "/Game/Enemies/Enums/E_MovementSpeed Enum" :default "NewEnumerator0"))
  (set `CharacterMovementComponent.MaxWalkSpeed` (select `/Game/Enemies/Enums/E_MovementSpeed` MovementSpeed :`NewEnumerator1` 200.0 :`NewEnumerator2` 500.0 :`NewEnumerator3` 700.0 :!type "Float (single-precision)") (`self.CharacterMovement`)))

(fn `GetIdealRange`
  (returns (AttackRange :type "Float (double-precision)"))
  (return 0.0))

(fn `GetPatrolRoute`
  (returns (PatrolRoute :type "/Game/Enemies/Patrol/BP_PatrolRoute Object Reference"))
  (return (`self.PatrolRoute`)))

(fn `UserConstructionScript`
  (`SkinnedMeshComponent.SetLeaderPoseComponent` (`self.Legs`) (`self.Mesh`) false false)
  (`SkinnedMeshComponent.SetLeaderPoseComponent` (`self.Hands`) (`self.Mesh`) false false)
  (`SkinnedMeshComponent.SetLeaderPoseComponent` (`self.Head`) (`self.Mesh`) false false)
  (`SkinnedMeshComponent.SetLeaderPoseComponent` (`self.Feet`) (`self.Mesh`) false false))