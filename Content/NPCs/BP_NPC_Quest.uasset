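; Quest-giver NPC that plays dialogue, then opens a quest panel.
; Interaction, also triggered automatically seven seconds after BeginPlay, freezes player movement and steps through Dialogues in WB_QuestDialogue.
; After the last line it swaps in a short repeat greeting and shows WB_Quest, filled from Quests, with the mouse cursor on.
; The panel gets an NPC reference; CloseWidget or interacting again removes it, restoring game input and walking.
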(event `self.ReceiveBeginPlay`
  (bind _returnvalue (`GameplayStatics.GetPlayerController` 0))
  (bind _dialoguewidget (`self.DialogueWidget`))
  (bind _dialogues (`self.Dialogues`))
  (`parent.ReceiveBeginPlay`)
  (`KismetSystemLibrary.Delay` 7.0)
  (if (`self.IsQuestWBActive`) :!label _label
    (`Widget.RemoveFromParent` (`self.QuestWidget`) :!label _label_2)
    (set `self.QuestWidget` null)
    (set `self.IsQuestWBActive` false)
    (set `PlayerController.bShowMouseCursor` false _returnvalue)
    (`WidgetBlueprintLibrary.SetInputMode_GameOnly` _returnvalue)
    (`CharacterMovementComponent.SetMovementMode` (`Character.CharacterMovement` (`GameplayStatics.GetPlayerCharacter` 0)) "MOVE_Walking" 0)
    (else
      (`CharacterMovementComponent.DisableMovement` (`Character.CharacterMovement` (`GameplayStatics.GetPlayerCharacter` 0)))
      (if (`self.IsDialogueActive`)
        (set `TextBlock.Text` (`KismetTextLibrary.Conv_StringToText` (`|GetArrayItem` (`self.Dialogues`) (`self.DialoguesIndex`))) (`/Game/UI/Widgets/WB_QuestDialogue.DialogueText` _dialoguewidget))
        (bind _result (`/Engine/EditorBlueprintResources/StandardMacros.IncrementInt` (`self.DialoguesIndex`))
          (:`  `
            (if (< (`KismetArrayLibrary.Array_Length` (`self.Dialogues`)) _result)
              (`Widget.RemoveFromParent` _dialoguewidget)
              (set `self.DialoguesIndex` 0)
              (`KismetArrayLibrary.Array_Clear` _dialogues)
              (`KismetArrayLibrary.Array_Add` _dialogues "조사는 잘 되고 있나?")
              (set `self.IsDialogueActive` false)
              (`self.ShowQuestPanel`))))
        (else
          (bind _returnvalue_2 (`|CreateWidget` "/Game/UI/Widgets/WB_QuestDialogue.WB_QuestDialogue_C"))
          (bind _output_get (set `self.DialogueWidget` _returnvalue_2))
          (set `TextBlock.Text` (`KismetTextLibrary.Conv_StringToText` (`|GetArrayItem` (`self.Dialogues`))) (`/Game/UI/Widgets/WB_QuestDialogue.DialogueText` _output_get))
          (`UserWidget.AddToViewport` _output_get 0)
          (set `self.IsDialogueActive` true)
          (`/Engine/EditorBlueprintResources/StandardMacros.IncrementInt` (`self.DialoguesIndex`)))))))

(event `self.CloseWidget`
  (goto _label_2))

(event `/Game/GameSystems/BPI_Interaction.InteractWith`
  (goto _label))

(event `ShowQuestPanel`
  (bind _returnvalue (`GameplayStatics.GetPlayerController` 0))
  (bind _questwidget (`self.QuestWidget`))
  (bind _returnvalue_2 (`|CreateWidget` "/Game/UI/Widgets/WB_Quest.WB_Quest_C"))
  (bind _output_get (set `self.QuestWidget` _returnvalue_2))
  (`UserWidget.AddToViewport` _output_get 0)
  (set `self.IsQuestWBActive` true)
  (set `PlayerController.bShowMouseCursor` true _returnvalue)
  (`WidgetBlueprintLibrary.SetInputMode_GameAndUIEx` _returnvalue (`self.QuestWidget`))
  (for _array_element (`self.Quests`)
    (`/Game/UI/Widgets/WB_Quest.Add Quest` _questwidget _array_element)
    (set `/Game/UI/Widgets/WB_Quest.NPC_ref` self _questwidget)))

(fn `UserConstructionScript`
  (`parent.UserConstructionScript`))