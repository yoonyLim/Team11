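; BP_NPC_Villager_E is a villager NPC that shows sequential dialogue lines when interacted with.
; Interactwith disables player movement, opens a WB_QuestDialogue widget on first use, and advances through the Dialogues array on later calls.
; Once the index passes the array's end, it removes the widget, resets dialogue state and restores walking.
; The construction script makes the modular body-part meshes follow the main Mesh's pose through leader pose components.
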(event `self.InteractWith`
  (bind _dialoguewidget (`self.DialogueWidget`))
  (bind _charactermovement (`Character.CharacterMovement` (`GameplayStatics.GetPlayerCharacter` 0)))
  (`CharacterMovementComponent.DisableMovement` _charactermovement)
  (if (`self.IsDialogueActive`)
    (set `TextBlock.Text` (`KismetTextLibrary.Conv_StringToText` (`|GetArrayItem` (`self.Dialogues`) (`self.DialoguesIndex`))) (`/Game/UI/Widgets/WB_QuestDialogue.DialogueText` _dialoguewidget))
    (bind _result (`/Engine/EditorBlueprintResources/StandardMacros.IncrementInt` (`self.DialoguesIndex`))
      (:`  `
        (if (< (`KismetArrayLibrary.Array_Length` (`self.Dialogues`)) _result)
          (`Widget.RemoveFromParent` _dialoguewidget)
          (set `self.DialoguesIndex` 0)
          (set `self.IsDialogueActive` false)
          (`CharacterMovementComponent.SetMovementMode` _charactermovement "MOVE_Walking" 0))))
    (else
      (bind _returnvalue (`|CreateWidget` "/Game/UI/Widgets/WB_QuestDialogue.WB_QuestDialogue_C"))
      (bind _output_get (set `self.DialogueWidget` _returnvalue))
      (set `TextBlock.Text` (`KismetTextLibrary.Conv_StringToText` (`|GetArrayItem` (`self.Dialogues`))) (`/Game/UI/Widgets/WB_QuestDialogue.DialogueText` _output_get))
      (`UserWidget.AddToViewport` _output_get 0)
      (set `self.IsDialogueActive` true)
      (`/Engine/EditorBlueprintResources/StandardMacros.IncrementInt` (`self.DialoguesIndex`)))))

(fn `UserConstructionScript`
  (`SkinnedMeshComponent.SetLeaderPoseComponent` (`self.Hat`) (`self.Mesh`) false false)
  (`SkinnedMeshComponent.SetLeaderPoseComponent` (`self.Legs`) (`self.Mesh`) false false)
  (`SkinnedMeshComponent.SetLeaderPoseComponent` (`self.Hands`) (`self.Mesh`) false false)
  (`SkinnedMeshComponent.SetLeaderPoseComponent` (`self.Feet`) (`self.Mesh`) false false)
  (`SkinnedMeshComponent.SetLeaderPoseComponent` (`self.Head`) (`self.Mesh`) false false))