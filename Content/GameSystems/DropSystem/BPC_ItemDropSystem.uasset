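; BPC_ItemDropSystem is a component that spawns item drops for its owning actor when DropItem is called.
; It looks up the owner's row in DT_ItemDrop, using the owner's class display name as the row name.
; Every class in that row's CommonItems is spawned with no random roll, slightly below the owner's location and spaced evenly along world Y by array index.
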(event `DropItem`
  (bind _returnvalue (`self.GetOwner`))
  (bind (_returnvalue_x _returnvalue_y _returnvalue_z) (`KismetMathLibrary.BreakVector` (`Actor.K2_GetActorLocation` _returnvalue)))
  (bind _returnvalue_2 (`|GetDataTableRow` "/Game/GameSystems/DropSystem/DT_ItemDrop.DT_ItemDrop" (`KismetStringLibrary.Conv_StringToName` (`KismetSystemLibrary.GetClassDisplayName` (`GameplayStatics.GetObjectClass` _returnvalue))))
    (:`then`
      (for (_array_element _array_index) (`.CommonItems_11_CD792D6446B91B3557030D9B2DECF835` (break `/Game/GameSystems/DropSystem/F_EnemyItemDrop` _returnvalue_2))
        (`|SpawnActorFromClass` _array_element (`KismetMathLibrary.MakeTransform` (`KismetMathLibrary.MakeVector` _returnvalue_x (+ (* _array_index 100) _returnvalue_y) (+ _returnvalue_z -50.0))) "Undefined" "MultiplyWithRoot" _returnvalue null)))))