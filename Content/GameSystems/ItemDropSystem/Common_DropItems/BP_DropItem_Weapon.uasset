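; BP_DropItem_Weapon is an interactable weapon drop that takes on the look of an enemy's weapon.
; On BeginPlay, if its owner is a BP_Enemy_Base, it copies the static mesh from that enemy's weapon onto SMWeapon, then runs the parent's BeginPlay.
; On interaction it simply destroys itself, with no item granting in this graph.
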(event `self.BP_InteractableObject.On Interacted`
  (`self.K2_DestroyActor`))

(event `self.ReceiveBeginPlay`
  (bind _asbp_enemy_base (cast `/Game/Enemies/BPs/BP_Enemy_Base` (`self.GetOwner`))
    (:`then`
      (`StaticMeshComponent.SetStaticMesh` (`self.SM_Weapon`) (`StaticMeshComponent.StaticMesh` (`self.GetComponentByClass` (`/Game/Enemies/BPs/BP_Enemy_Base.Weapon` _asbp_enemy_base) "/Script/Engine.StaticMeshComponent"))))
    (:`CastFailed`
      _))
  (`parent.ReceiveBeginPlay`))

(fn `UserConstructionScript`
  (`parent.UserConstructionScript`))