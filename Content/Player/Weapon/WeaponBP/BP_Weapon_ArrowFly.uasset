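; Flying arrow weapon Blueprint that damages what it hits and sticks into the enemy it touches.
; Every Tick it calls DetectHit with a fixed damage and the Player, then checks whether TouchedEnemy is valid.
; While that is valid, it stops projectile movement, zeroes gravity, attaches to the enemy keeping world transform, and destroys itself after a short Delay.
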(event `self.ReceiveTick`
  (params (DeltaSeconds :type "Float (single-precision)"))
  (bind _projectilemovement (`self.ProjectileMovement`))
  (`self.DetectHit` 20.0 (`self.Player`))
  (`/Engine/EditorBlueprintResources/StandardMacros.IsValid` (`self.TouchedEnemy`)
    (:`Is Valid`
      (`MovementComponent.StopMovementImmediately` _projectilemovement)
      (set `ProjectileMovementComponent.ProjectileGravityScale` 0.0 _projectilemovement)
      (`self.K2_AttachToActor` (`self.TouchedEnemy`) "None" "KeepWorld" "KeepWorld" "KeepWorld")
      (`KismetSystemLibrary.Delay` 5.0)
      (`self.K2_DestroyActor`))))

(fn `UserConstructionScript`
  (`parent.UserConstructionScript`))