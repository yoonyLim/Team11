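; Base weapon actor that applies sword hit damage to enemies.
; When DetectHit is called while CanInflictDamage is set, it damages every BP_Enemy_Base overlapping SwordMesh, naming the passed Player as damage causer.
; A hit clears CanInflictDamage, sets the Player's IsDamage flag and stores the enemy in TouchedEnemy.
; Detection runs only on that call, as Tick and overlap events are empty, and nothing here re-arms the damage flag.
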(event `DetectHit`
  (params (Damage :type "Float (double-precision)") (Player :type "/Game/Player/BluePrints/BP_Player Object Reference"))
  (if (`self.CanInflictDamage?`)
    (for _array_element (`PrimitiveComponent.GetOverlappingActors` (`self.SwordMesh`) "/Script/Engine.Actor")
      (bind _asbp_enemy_base (cast `/Game/Enemies/BPs/BP_Enemy_Base` _array_element))
      (`/Game/GameSystems/DamageSystem/BPI_Damageable.TakeDamage` _asbp_enemy_base (make `/Game/GameSystems/DamageSystem/F_DamageInfo` Damage "NewEnumerator3" "NewEnumerator0" false true) Player)
      (set `self.CanInflictDamage?` false)
      (set `/Game/Player/BluePrints/BP_Player.IsDamage?` true Player)
      (set `self.TouchedEnemy` _asbp_enemy_base))))

(fn `UserConstructionScript`)