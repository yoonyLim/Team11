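; First boss enemy Blueprint, a saber-wielding character with its own boss health bar, built on a parent enemy class.
; BeginPlay creates the bar, seeds the damage component's health and spawns the saber on a carry socket.
; Equip and unequip montages move the saber between sockets on notifies, while attacks play one of three random montages.
; Death removes the bar and drops an item; hat and mask follow the body via leader pose.
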(event `self.ReceiveBeginPlay`
  (bind _maxhealth (`self.MaxHealth`))
  (bind _bpc_damagesystem (`self.BPC_DamageSystem`))
  ;[1 1 1] HP Widget Ready
  (`WidgetComponent.SetWidget` (`self.WB_HealthBar`) null)
  (bind _returnvalue (`|CreateWidget` "/Game/UI/Widgets/WB_BossHealthBar.WB_BossHealthBar_C" null null))
  (bind _output_get (set `self.BossHealthBar` _returnvalue))
  (bind _leveltext (`/Game/UI/Widgets/WB_BossHealthBar.LevelText` _output_get))
  (set `TextBlock.Text` (`KismetTextLibrary.Conv_StringToText` (`KismetStringLibrary.Concat_StrStr` (`KismetTextLibrary.Conv_TextToString` (`TextBlock.Text` _leveltext)) (`KismetStringLibrary.Conv_IntToString` (`self.Level`)))) _leveltext)
  (set `TextBlock.Text` (`self.Name`) (`/Game/UI/Widgets/WB_BossHealthBar.EnemyName` _output_get))
  (set `/Game/GameSystems/DamageSystem/BPC_DamageSystem.MaxHealth` _maxhealth _bpc_damagesystem)
  (set `/Game/GameSystems/DamageSystem/BPC_DamageSystem.Health` _maxhealth _bpc_damagesystem)
  (`self.UpdateHP`)
  ;[1 1 1] Weapon Ready
  (bind _returnvalue_2 (`|SpawnActorFromClass` "/Game/Enemies/Weapons/BP_Enemy_Weapon_Saber.BP_Enemy_Weapon_Saber_C" (`self.GetTransform`) "Undefined" "MultiplyWithRoot" self null))
  (bind _output_get_2 (set `self.Weapon` _returnvalue_2))
  (`self.K2_AttachToComponent` _output_get_2 (`self.Mesh`) "enemy_weapon_carry_socket" "SnapToTarget" "SnapToTarget" "SnapToTarget" true))

(event `/Game/Enemies/Interfaces/BPI_Enemy.EquipWeapon`
  (bind _mesh (`self.Mesh`))
  ;[1 1 1] Equip/Unequip Weapon
  (bind _notifyname (`|PlayMontage` _mesh (`self.MT_EquipWeapon`))
    (:`OnCompleted`
      (`self.OnWeaponEquipped`))
    (:`OnNotifyBegin`
      (switch `name` _notifyname
        (:`Unsheathe`
          (bind _returnvalue (`self.K2_AttachToComponent` (`self.Weapon`) _mesh "enemy_weapon_equip_socket" "SnapToTarget" "SnapToTarget" "SnapToTarget" true))
          (set `self.IsWeaponEquipped` _returnvalue))))))

(event `/Game/Enemies/Interfaces/BPI_Enemy.UnequipWeapon`
  (bind _mesh (`self.Mesh`))
  ;[1 1 1] Equip/Unequip Weapon
  (bind _notifyname (`|PlayMontage` _mesh (`self.MT_UnequipWeapon`))
    (:`OnCompleted`
      (`self.OnWeaponUnEquipped`))
    (:`OnNotifyBegin`
      (switch `name` _notifyname
        (:`Sheathe`
          (`self.K2_AttachToComponent` (`self.Weapon`) _mesh "enemy_weapon_carry_socket" "SnapToTarget" "SnapToTarget" "SnapToTarget" true)
          (set `self.IsWeaponEquipped` false))))))

(event `/Game/Enemies/Interfaces/BPI_Enemy.Attack`
  (params (AttackTarget :type "Actor Object Reference"))
  (bind _mesh (`self.Mesh`))
  (`parent.Attack` AttackTarget)
  (switch `int` (`KismetMathLibrary.RandomInteger` 3)
    (:`0`
      (`|PlayMontage` _mesh (`self.MT_Attack`)
        (:`OnCompleted`
          _)
        (:`OnInterrupted`
          _)))
    (:`1`
      (`|PlayMontage` _mesh (`self.MT_Attack_A`)
        (:`OnCompleted`
          _)
        (:`OnInterrupted`
          _)))
    (:`2`
      (`|PlayMontage` _mesh (`self.MT_Attack_B`)
        (:`OnCompleted`
          _)
        (:`OnInterrupted`
          _))))
  (`self.OnAttackEnded`))

(event `self.BPC_DamageSystem.OnDeath`
  (`Widget.RemoveFromParent` (`self.BossHealthBar`))
  (`/Game/GameSystems/ItemDropSystem/BPC_ItemDropSystem.DropItem` (`self.BPC_DropSystem`)))

(fn `UpdateHP`
  (bind _bpc_damagesystem (`self.BPC_DamageSystem`))
  (bind _bosshealthbar (`self.BossHealthBar`)
    (:`then`
      (`/Game/UI/Widgets/WB_BossHealthBar.UpdateHealthPercentage` _bosshealthbar (`/Game/GameSystems/DamageSystem/BPC_DamageSystem.Health` _bpc_damagesystem) (`/Game/GameSystems/DamageSystem/BPC_DamageSystem.MaxHealth` _bpc_damagesystem)))
    (:`else`)))

(fn `UserConstructionScript`
  (`parent.UserConstructionScript`)
  (`SkinnedMeshComponent.SetLeaderPoseComponent` (`self.Hat`) (`self.Mesh`) false false)
  (`SkinnedMeshComponent.SetLeaderPoseComponent` (`self.Mask`) (`self.Mesh`) false false))