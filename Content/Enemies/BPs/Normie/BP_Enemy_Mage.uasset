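; Mage enemy that spawns a staff into its hand socket on BeginPlay and fights at range with a beam.
; Attack plays a montage whose notify spawns BP_MageBeam above the actor at the given target, while completion signals attack end.
; Equip and unequip only set a flag and notify next tick, as their montage logic is disconnected.
; Modular body meshes follow the main mesh via leader pose, and GetIdealRange supplies its preferred distance.
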(event `self.ReceiveBeginPlay`
  (`parent.ReceiveBeginPlay`)
  (bind _returnvalue (`|SpawnActorFromClass` "/Game/Enemies/Weapons/BP_Enemy_Weapon_Staff.BP_Enemy_Weapon_Staff_C" (`self.GetTransform`) "Undefined" "MultiplyWithRoot" self null))
  (bind _output_get (set `self.Weapon` _returnvalue))
  (`self.K2_AttachToComponent` _output_get (`self.Mesh`) "enemy_weapon_equip_socket" "SnapToTarget" "SnapToTarget" "SnapToTarget" true))

(event `self.EquipWeapon`
  ;[1 1 1] Equip/Unequip Weapon
  (set `self.IsWeaponEquipped` true)
  (`KismetSystemLibrary.DelayUntilNextTick`)
  (`self.OnWeaponEquipped`))

(event `self.UnequipWeapon`
  ;[1 1 1] Equip/Unequip Weapon
  (set `self.IsWeaponEquipped` false)
  (`KismetSystemLibrary.DelayUntilNextTick`)
  (`self.OnWeaponUnEquipped`))

(event `/Game/Enemies/Interfaces/BPI_Enemy.Attack`
  (params (AttackTarget :type "Actor Object Reference"))
  (bind _returnvalue (`self.GetTransform`))
  (bind _notifyname (`|PlayMontage` (`self.Mesh`) (`self.MT_Attack`))
    (:`OnCompleted`
      (`self.OnAttackEnded`))
    (:`OnNotifyBegin`
      (switch `name` _notifyname
        (:`Spawn`
          (`|SpawnActorFromClass` "/Game/Enemies/Projectiles/BP_MageBeam.BP_MageBeam_C" (`KismetMathLibrary.MakeTransform` (`KismetMathLibrary.MakeVector` (.x (.location _returnvalue)) (.y (.location _returnvalue)) (+ (.z (.location _returnvalue)) 100.0)) (.rotation _returnvalue) (.scale _returnvalue)) "Undefined" "MultiplyWithRoot" self (0.0 0.0 0.0) AttackTarget null))))))

(fn `GetIdealRange`
  (returns (AttackRange :type "Float (double-precision)"))
  (return 600.0))

(fn `UserConstructionScript`
  (`parent.UserConstructionScript`)
  (`SkinnedMeshComponent.SetLeaderPoseComponent` (`self.Legs`) (`self.Mesh`) false false)
  (`SkinnedMeshComponent.SetLeaderPoseComponent` (`self.Hands`) (`self.Mesh`) false false)
  (`SkinnedMeshComponent.SetLeaderPoseComponent` (`self.Head`) (`self.Mesh`) false false)
  (`SkinnedMeshComponent.SetLeaderPoseComponent` (`self.Feet`) (`self.Mesh`) false false)
  (`SkinnedMeshComponent.SetLeaderPoseComponent` (`self.Hat`) (`self.Mesh`) false false)
  (`SkinnedMeshComponent.SetLeaderPoseComponent` (`self.Hair`) (`self.Mesh`) false false))