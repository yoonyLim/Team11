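; Melee enemy Blueprint that carries a staff weapon and plays equip, unequip and attack montages.
; On BeginPlay it spawns the staff on the carry socket; montage notifies in both equip and unequip attach it to the equip socket and update the equipped flag.
; Montage completion calls the matching equipped, unequipped or attack-ended notification.
; The construction script makes the modular body meshes follow the main mesh's pose.
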(event `self.ReceiveBeginPlay`
  (`parent.ReceiveBeginPlay`)
  (bind _returnvalue (`|SpawnActorFromClass` "/Game/Enemies/Weapons/BP_Enemy_Weapon_Staff.BP_Enemy_Weapon_Staff_C" (`self.GetTransform`) "Undefined" "MultiplyWithRoot" self null))
  (bind _output_get (set `self.Weapon` _returnvalue))
  (`self.K2_AttachToComponent` _output_get (`self.Mesh`) "enemy_weapon_carry_socket" "SnapToTarget" "SnapToTarget" "SnapToTarget" true))

(event `/Game/Enemies/Interfaces/BPI_Enemy.UnequipWeapon`
  (bind _mesh (`self.Mesh`))
  ;[1 1 1] Equip/Unequip Weapon
  (bind _notifyname (`|PlayMontage` _mesh (`self.MT_UnequipWeapon`))
    (:`OnCompleted`
      (`self.OnWeaponUnEquipped`))
    (:`OnNotifyBegin`
      (switch `name` _notifyname
        (:`Sheathe`
          (`self.K2_AttachToComponent` (`self.Weapon`) _mesh "enemy_weapon_equip_socket" "SnapToTarget" "SnapToTarget" "SnapToTarget" true)
          (set `self.IsWeaponEquipped` false))))))

(event `/Game/Enemies/Interfaces/BPI_Enemy.EquipWeapon`
  (bind _mesh (`self.Mesh`))
  ;[1 1 1] Equip/Unequip Weapon
  (bind _notifyname (`|PlayMontage` _mesh (`self.MT_EquipWeapon`))
    (:`OnCompleted`
      (`self.OnWeaponEquipped`))
    (:`OnNotifyBegin`
      (switch `name` _notifyname
        (:`Unsheathe`
          (bind _returnvalue (`self.K2_AttachToComponent` (`self.Weapon`) _mesh "enemy_weapon_equip_socket" "SnapToTarget" "SnapToTarget" "SnapToTarget" true))
          (set `self.IsWeaponEquipped` _returnvalue))))))

(event `/Game/Enemies/Interfaces/BPI_Enemy.Attack`
  (`|PlayMontage` (`self.Mesh`) (`self.MT_Attack`)
    (:`OnCompleted`
      (`self.OnAttackEnded`))))

(fn `UserConstructionScript`
  (`parent.UserConstructionScript`)
  (`SkinnedMeshComponent.SetLeaderPoseComponent` (`self.Legs`) (`self.Mesh`) false false)
  (`SkinnedMeshComponent.SetLeaderPoseComponent` (`self.Hands`) (`self.Mesh`) false false)
  (`SkinnedMeshComponent.SetLeaderPoseComponent` (`self.Head`) (`self.Mesh`) false false)
  (`SkinnedMeshComponent.SetLeaderPoseComponent` (`self.Feet`) (`self.Mesh`) false false))