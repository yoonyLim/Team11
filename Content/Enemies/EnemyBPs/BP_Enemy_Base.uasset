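; Base enemy character that routes damage and health through a damage system component and shows health on a widget rotated toward the player camera each tick.
; Hits flash an overlay material on a short timer and classify the attacker's direction by relative yaw, though no directional response is wired.
; Death enables ragdoll physics before delayed destruction.
; It also exposes movement speed presets and combat getters, with dead and invincible checks hardcoded to false.
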(event `self.ReceiveBeginPlay`
  (bind _bpc_damagesystem (`self.BPC_DamageSystem`))
  (bind _asw_health_bar (cast `/Game/GameSystems/DamageSystem/W_HealthBar` (`WidgetComponent.GetWidget` (`self.W_HealthBar`))))
  (bind _output_get (set `self.HealthBar` _asw_health_bar))
  (`/Game/GameSystems/DamageSystem/W_HealthBar.UpdateHealthPercentage` _output_get (`/Game/GameSystems/DamageSystem/BPC_DamageSystem.Health` _bpc_damagesystem) (`/Game/GameSystems/DamageSystem/BPC_DamageSystem.MaxHealth` _bpc_damagesystem)))

(event `self.ReceiveTick`
  (params (DeltaSeconds :type "Float (single-precision)"))
  (`SceneComponent.K2_SetWorldRotation` (`self.W_HealthBar`) (`KismetMathLibrary.FindLookAtRotation` (`self.K2_GetActorLocation`) (`PlayerCameraManager.GetCameraLocation` (`GameplayStatics.GetPlayerCameraManager` 0))) false false))

(event `self.BPC_DamageSystem.OnDamageResponse`
  (params (DamageResponse :type "/Game/GameSystems/DamageSystem/E_DamageResponse Enum" :default "NewEnumerator0") (DamageCauser :type "Actor Object Reference"))
  (`self.PlayHitEffect`)
  (bind _hitdirection (`self.GetHitDirection` DamageCauser))
  (switch `/Game/Enemies/Enums/E_HitDirection` _hitdirection))

(event `self.BPC_DamageSystem.OnDeath`
  (bind _mesh (`self.Mesh`))
  (`self.PlayHitEffect`)
  (`PrimitiveComponent.SetSimulatePhysics` _mesh true)
  (`PrimitiveComponent.SetCollisionEnabled` _mesh "QueryAndPhysics")
  (`KismetSystemLibrary.Delay` 3.0)
  (`self.K2_DestroyActor`))

(event `ResetOverlayMaterial`
  (`MeshComponent.SetOverlayMaterial` (`self.Mesh`) null))

(event `/Game/Enemies/Interfaces/BPI_Enemy.SetMovementSpeed`
  (params (MovementSpeed :type "/Game/Enemies/Enums/E_EnemyMovementSpeed Enum" :default "NewEnumerator0"))
  (set `CharacterMovementComponent.MaxWalkSpeed` (select `/Game/Enemies/Enums/E_EnemyMovementSpeed` MovementSpeed :`NewEnumerator1` 200.0 :`NewEnumerator2` 400.0 :`NewEnumerator3` 700.0 :!type "Float (single-precision)") (`self.CharacterMovement`)))

(fn `GetCurrentHealth`
  (returns (Health :type "Float (double-precision)"))
  (return (`/Game/GameSystems/DamageSystem/BPC_DamageSystem.Health` (`self.BPC_DamageSystem`))))

(fn `GetHitDirection`
  (params (Attacker :type "Actor Object Reference"))
  (returns (HitDirection :type "/Game/Enemies/Enums/E_HitDirection Enum"))
  (bind (_returnvalue_roll _returnvalue_pitch _returnvalue_yaw) (`KismetMathLibrary.BreakRotator` (`KismetMathLibrary.FindRelativeLookAtRotation` (`self.GetTransform`) (`self.K2_GetActorLocation` Attacker))))
  (if (`KismetMathLibrary.InRange_FloatFloat` _returnvalue_yaw -45.0 45.0)
    (return "NewEnumerator0")
    (elif (`KismetMathLibrary.InRange_FloatFloat` _returnvalue_yaw 45.0 135.0 false)
      (return "NewEnumerator2")
      (elif (`KismetMathLibrary.InRange_FloatFloat` _returnvalue_yaw -135.0 -45.0 true false)
        (return "NewEnumerator3")
        (else
          (return "NewEnumerator1"))))))

(fn `GetIdealRange`
  (returns (AttackRange :type "Float (double-precision)"))
  (return (`self.AttackRange`)))

(fn `GetIsDead`
  (returns (IsDead :type Boolean))
  (return false))

(fn `GetIsInvincible`
  (returns (IsInvincible :type Boolean))
  (return false))

(fn `GetMaxHealth`
  (returns (MaxHealth :type "Float (double-precision)"))
  (return (`/Game/GameSystems/DamageSystem/BPC_DamageSystem.MaxHealth` (`self.BPC_DamageSystem`))))

(fn `TakeDamage`
  (params (DamageInfo :type "/Game/GameSystems/DamageSystem/F_DamageInfo Structure") (`Damage Causer` :type "Actor Object Reference"))
  (returns (WasDamaged :type Boolean))
  (bind _bpc_damagesystem (`self.BPC_DamageSystem`))
  (bind _wasdamaged (`/Game/GameSystems/DamageSystem/BPC_DamageSystem.TakeDamage` (`self.BPC_DamageSystem`) DamageInfo `Damage Causer`))
  (`/Game/GameSystems/DamageSystem/W_HealthBar.UpdateHealthPercentage` (`self.HealthBar`) (`/Game/GameSystems/DamageSystem/BPC_DamageSystem.Health` _bpc_damagesystem) (`/Game/GameSystems/DamageSystem/BPC_DamageSystem.MaxHealth` _bpc_damagesystem))
  (return _wasdamaged))

(fn `UserConstructionScript`)