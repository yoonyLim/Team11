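; Enemy saber projectile that spins as it exists in the world and damages the player on contact.
; A timeline that restarts itself on finish drives the yaw of RotationPoint for continuous spinning, and the actor expires after a short fixed lifetime.
; When its capsule overlaps BP_Player, it applies damage, calls OnProjectileImpact, disables collision and destroys itself after a brief delay.
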(event `self.ReceiveBeginPlay`
  (`parent.ReceiveBeginPlay`)
  (`self.Spin`)
  (`KismetSystemLibrary.Delay` 3.0)
  (`self.K2_DestroyActor`))

(event `Spin`
  (bind (_returnvalue_roll _returnvalue_pitch) (`KismetMathLibrary.BreakRotator` (`SceneComponent.K2_GetComponentRotation` (`self.RotationPoint`))))
  (bind (_direction _z_rotation) (`Timeline|RotationTimeline` :!via `PlayFromStart`)
    (:`Update`
      (`SceneComponent.K2_SetWorldRotation` (`self.RotationPoint`) (`KismetMathLibrary.MakeRotator` _returnvalue_roll _returnvalue_pitch _z_rotation) false false))
    (:`Finished`
      (`self.Spin`))))

(event `self.CapsuleCollision.OnComponentBeginOverlap`
  (params (OverlappedComponent :type "PrimitiveComponent Object Reference") (OtherActor :type "Actor Object Reference") (OtherComp :type "PrimitiveComponent Object Reference") (OtherBodyIndex :type Integer) (bFromSweep :type Boolean) (SweepResult :type "HitResult Structure (by ref)"))
  (bind _asbp_player (cast `/Game/Player/BluePrints/BP_Player` OtherActor))
  (`/Game/Player/BluePrints/BP_Player.TakeDamage` _asbp_player (make `/Game/GameSystems/DamageSystem/F_DamageInfo` 10.0 "NewEnumerator2") self)
  (`self.OnProjectileImpact` OtherActor SweepResult)
  (`PrimitiveComponent.SetCollisionEnabled` (`self.CapsuleCollision`) "NoCollision")
  (`KismetSystemLibrary.Delay` 0.2)
  (`self.K2_DestroyActor`))

(fn `UserConstructionScript`
  (`parent.UserConstructionScript`))