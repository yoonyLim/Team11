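; Boss projectile that flies along a set direction and damages the player on overlap.
; The construction script applies speed and gravity to projectile movement, with optional homing on the target's root component.
; On BeginPlay it launches, turns its yaw toward the target, ignores its instigator or owner when moving, and expires after a short delay.
; Overlapping the player sends a damage message, disables capsule collision and destroys the projectile.
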(event `self.ReceiveBeginPlay`
  (bind _returnvalue (`self.GetInstigator`))
  (`self.Fly`)
  (`PrimitiveComponent.IgnoreActorWhenMoving` (`self.CapsuleCollision`) (select `bool` (`KismetSystemLibrary.IsValid` _returnvalue) :`false` (`self.GetOwner`) :`true` _returnvalue :!type "Actor Object Reference") true)
  (`KismetSystemLibrary.Delay` 3.0)
  (`self.K2_DestroyActor`))

(event `Fly`
  (bind (_returnvalue_roll _returnvalue_pitch _returnvalue_yaw) (`KismetMathLibrary.BreakRotator` (`KismetMathLibrary.FindLookAtRotation` (`self.K2_GetActorLocation`) (`self.K2_GetActorLocation` (`self.Target`)))))
  (set `MovementComponent.Velocity` (* (`self.Direction`) (`self.Speed`)) (`self.ProjectileMovement`))
  (`self.K2_SetActorRotation` (`KismetMathLibrary.MakeRotator` 0.0 0.0 _returnvalue_yaw)))

(event `self.CapsuleCollision.OnComponentBeginOverlap`
  (params (OverlappedComponent :type "PrimitiveComponent Object Reference") (OtherActor :type "Actor Object Reference") (OtherComp :type "PrimitiveComponent Object Reference") (OtherBodyIndex :type Integer) (bFromSweep :type Boolean) (SweepResult :type "HitResult Structure (by ref)"))
  (bind _asbp_player (cast `/Game/Player/BluePrints/BP_Player` OtherActor))
  (message `/Game/GameSystems/DamageSystem/BPI_Damageable.TakeDamage` _asbp_player (make `/Game/GameSystems/DamageSystem/F_DamageInfo` (`self.DamageAmount`)) self)
  (`PrimitiveComponent.SetCollisionEnabled` (`self.CapsuleCollision`) "NoCollision")
  (`self.K2_DestroyActor`))

(fn `UserConstructionScript`
  (bind _projectilemovement (`self.ProjectileMovement`))
  (bind _speed (`self.Speed`))
  (set `ProjectileMovementComponent.InitialSpeed` _speed _projectilemovement)
  (set `ProjectileMovementComponent.MaxSpeed` _speed _projectilemovement)
  (set `ProjectileMovementComponent.ProjectileGravityScale` (`self.Gravity`) _projectilemovement)
  (`self.Target`
    (:`then`
      (if (`self.IsHoming`)
        (set `ProjectileMovementComponent.bIsHomingProjectile` true _projectilemovement)
        (set `ProjectileMovementComponent.HomingTargetComponent` (`Actor.RootComponent` (`self.Target`)) _projectilemovement)))
    (:`else`)))