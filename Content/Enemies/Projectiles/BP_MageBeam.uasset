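; Mage beam attack actor that charges for a second, then fires at where its target stood when the charge began.
; BeginPlay spawns a Niagara ball, snapshots the target location, then spawns the trail and sphere-traces along that line to damage the player.
; Tick keeps the ball on the actor and fast-forwards the trail with AdvanceSimulation.
; The trail and actor are destroyed a second after firing.
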(event `self.ReceiveBeginPlay`
  (bind _targetlocation (`self.TargetLocation`))
  (bind _returnvalue (`NiagaraFunctionLibrary.SpawnSystemAtLocation` "/Game/Asset/ACTION/Enemy/Boss/Niagara/Ball/NS_Boss_Skill_2_1_Ball.NS_Boss_Skill_2_1_Ball" (`self.SpawnLocation`)))
  (set `self.TargetLocation` (`self.K2_GetActorLocation` (`self.AttackTarget`)))
  (`KismetSystemLibrary.Delay` 1.0)
  (bind _returnvalue_2 (`SceneComponent.K2_GetComponentLocation` _returnvalue))
  (bind _returnvalue_3 (`NiagaraFunctionLibrary.SpawnSystemAtLocation` "/Game/Asset/ACTION/Enemy/Boss/Niagara/Ball/NS_Boss_Skill_2_2_Trail.NS_Boss_Skill_2_2_Trail" _returnvalue_2 (`KismetMathLibrary.FindLookAtRotation` _targetlocation _returnvalue_2) (3.0 3.0 3.0)))
  (bind (_outhit _returnvalue_4) (`KismetSystemLibrary.SphereTraceSingle` _returnvalue_2 (+ (* (`KismetMathLibrary.GetForwardVector` (`KismetMathLibrary.FindLookAtRotation` _returnvalue_2 _targetlocation)) 5000.0) _returnvalue_2) 10.0 "TraceTypeQuery2"))
  (if _returnvalue_4
    (bind _asbp_player (cast `/Game/Player/BluePrints/BP_Player` (`.HitActor` (`GameplayStatics.BreakHitResult` _outhit)))
      (:`then`
        (`/Game/GameSystems/DamageSystem/BPI_Damageable.TakeDamage` _asbp_player (make `/Game/GameSystems/DamageSystem/F_DamageInfo` 1.0 "NewEnumerator2") (`self.GetOwner`)))
      (:`CastFailed`
        _)))
  (`KismetSystemLibrary.Delay` 1.0)
  (`ActorComponent.K2_DestroyComponent` _returnvalue_3)
  (`self.K2_DestroyActor`))

(event `self.ReceiveTick`
  (params (DeltaSeconds :type "Float (single-precision)"))
  (`SceneComponent.K2_SetWorldLocation` (stale `self.ReceiveBeginPlay` _returnvalue) (`self.K2_GetActorLocation`) false false)
  (`/Engine/EditorBlueprintResources/StandardMacros.IsValid` (stale `self.ReceiveBeginPlay` _returnvalue_3)
    (:`Is Valid`
      (`NiagaraComponent.AdvanceSimulation` (stale `self.ReceiveBeginPlay` _returnvalue_3) 1 (* DeltaSeconds 4.0)))))

(fn `UserConstructionScript`)