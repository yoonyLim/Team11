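; Base Blueprint for enemy weapons that deals damage to the player on contact.
; DetectHit, when called with a damage amount, checks the actors overlapping the weapon mesh and applies TakeDamage to BP_Player, with the weapon's owner as causer.
; A CanInflictDamage flag gates the check and clears after a hit; this graph never re-enables it.
; The mesh's begin-overlap event is empty, and a random-damage branch is left disconnected.
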(event `self.SM_Weapon.OnComponentBeginOverlap`
  (params (OverlappedComponent :type "PrimitiveComponent Object Reference") (OtherActor :type "Actor Object Reference") (OtherComp :type "PrimitiveComponent Object Reference") (OtherBodyIndex :type Integer) (bFromSweep :type Boolean) (SweepResult :type "HitResult Structure (by ref)")))

(event `DetectHit`
  (params (Damage :type "Float (double-precision)"))
  (if (`self.CanInflictDamage`)
    (for _array_element (`PrimitiveComponent.GetOverlappingActors` (`self.SM_Weapon`) null)
      (bind _asbp_player (cast `/Game/Player/BluePrints/BP_Player` _array_element))
      (`/Game/GameSystems/DamageSystem/BPI_Damageable.TakeDamage` _asbp_player (make `/Game/GameSystems/DamageSystem/F_DamageInfo` Damage "NewEnumerator1") (`self.GetOwner`))
      (set `self.CanInflictDamage` false))))

(fn `UserConstructionScript`)