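; Base enemy Blueprint that delegates damage and health to a damage system component and shows health on a camera-facing widget bar.
; TakeDamage forwards to the component and refreshes the bar, while damage responses flash a hit overlay material briefly via a timer.
; On death it flashes, enables mesh physics and destroys itself after a delay.
; Heal, IsAttacking and IsDead are stubs returning default values.
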(event `self.ReceiveBeginPlay`
  (bind _bpc_damagesystem (`self.BPC_DamageSystem`))
  (bind _asw_health_bar (cast `/Game/GameSystems/DamageSystem/W_HealthBar` (`WidgetComponent.GetWidget` (`self.W_HealthBar`))))
  (set `self.HealthBar` _asw_health_bar)
  (`/Game/GameSystems/DamageSystem/W_HealthBar.UpdateHealthPercentage` (`self.HealthBar`) (`/Game/GameSystems/DamageSystem/BPC_DamageSystem.Health` _bpc_damagesystem) (`/Game/GameSystems/DamageSystem/BPC_DamageSystem.MaxHealth` _bpc_damagesystem)))

(event `self.ReceiveTick`
  (params (DeltaSeconds :type "Float (single-precision)"))
  (`SceneComponent.K2_SetWorldRotation` (`self.W_HealthBar`) (`KismetMathLibrary.FindLookAtRotation` (`self.K2_GetActorLocation`) (`PlayerCameraManager.GetCameraLocation` (`GameplayStatics.GetPlayerCameraManager` 0))) false false))

(event `self.BPC_DamageSystem.OnDamageResponse`
  (params (DamageResponse :type "/Game/GameSystems/DamageSystem/E_DamageResponse Enum" :default "NewEnumerator0") (DamageCauser :type "Actor Object Reference"))
  (`self.PlayHitAnim`))

(event `self.BPC_DamageSystem.OnDeath`
  (bind _mesh (`self.Mesh`))
  (`self.PlayHitAnim`)
  (`PrimitiveComponent.SetSimulatePhysics` _mesh true)
  (`PrimitiveComponent.SetCollisionEnabled` _mesh "QueryAndPhysics")
  (`KismetSystemLibrary.Delay` 3.0)
  (`self.K2_DestroyActor`))

(event `ResetOverlayMaterial`
  (`MeshComponent.SetOverlayMaterial` (`self.Mesh`) null))

(fn `GetCurrentHealth`
  (returns (Health :type "Float (double-precision)"))
  (return (`/Game/GameSystems/DamageSystem/BPC_DamageSystem.Health` (`self.BPC_DamageSystem`))))

(fn `GetMaxHealth`
  (returns (MaxHealth :type "Float (double-precision)"))
  (return (`/Game/GameSystems/DamageSystem/BPC_DamageSystem.MaxHealth` (`self.BPC_DamageSystem`))))

(fn `Heal`
  (params (Amount :type "Float (double-precision)"))
  (returns (NewHealth :type "Float (double-precision)"))
  (return 0.0))

(fn `IsAttacking`
  (returns (Attacking :type Boolean))
  (return false))

(fn `IsDead`
  (returns (Dead :type Boolean))
  (return false))

(fn `TakeDamage`
  (params (DamageInfo :type "/Game/GameSystems/DamageSystem/F_DamageInfo Structure") (`Damage Causer` :type "Actor Object Reference"))
  (returns (WasDamaged :type Boolean))
  (bind _bpc_damagesystem (`self.BPC_DamageSystem`))
  (bind _wasdamaged (`/Game/GameSystems/DamageSystem/BPC_DamageSystem.TakeDamage` (`self.BPC_DamageSystem`) DamageInfo `Damage Causer`))
  (`/Game/GameSystems/DamageSystem/W_HealthBar.UpdateHealthPercentage` (`self.HealthBar`) (`/Game/GameSystems/DamageSystem/BPC_DamageSystem.Health` _bpc_damagesystem) (`/Game/GameSystems/DamageSystem/BPC_DamageSystem.MaxHealth` _bpc_damagesystem))
  (return _wasdamaged))

(fn `UserConstructionScript`)