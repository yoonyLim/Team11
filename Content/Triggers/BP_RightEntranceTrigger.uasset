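; Entrance trigger volume that forces a conversation with a referenced NPC when the player walks into it.
; On player overlap it calls the NPC's interaction and snaps both control and character rotation to face that NPC.
; At BeginPlay it binds to the dialogue-end event of the NPC, cast to Guard A, and destroys itself when that fires.
; Its own Interactwith event forwards an interaction message to the NPC.
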(event `self.ReceiveBeginPlay`
  (bind _asbp_npc_guard_a (cast `/Game/NPCs/BP_NPC_Guard_A` (`self.NPC`)))
  (add `/Game/NPCs/BP_NPC_Guard_A.OnDialogueEnd` _asbp_npc_guard_a (delegate `DialogueEnd_Event`)))

(event `DialogueEnd_Event`
  (`self.K2_DestroyActor`))

(event `self.Box.OnComponentBeginOverlap`
  (params (OverlappedComponent :type "PrimitiveComponent Object Reference") (OtherActor :type "Actor Object Reference") (OtherComp :type "PrimitiveComponent Object Reference") (OtherBodyIndex :type Integer) (bFromSweep :type Boolean) (SweepResult :type "HitResult Structure (by ref)"))
  (bind _returnvalue (`GameplayStatics.GetPlayerCharacter` 0))
  (bind _returnvalue_2 (`KismetMathLibrary.FindLookAtRotation` (`self.K2_GetActorLocation` _returnvalue) (`self.K2_GetActorLocation` (`self.NPC`))))
  (cast `/Game/Player/BluePrints/BP_Player` OtherActor)
  (`/Game/GameSystems/BPI_Interaction.InteractWith` (`self.NPC`))
  (`Controller.SetControlRotation` (`GameplayStatics.GetPlayerController` 0) _returnvalue_2)
  (`self.K2_SetActorRotation` _returnvalue _returnvalue_2 false))

(event `/Game/GameSystems/BPI_Interaction.InteractWith`
  (message `/Game/GameSystems/BPI_Interaction.InteractWith` (`self.NPC`)))

(fn `UserConstructionScript`)