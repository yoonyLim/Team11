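; BP_RiddlerTrigger is a one-shot box trigger that plays a cutscene, then starts an interaction with an NPC.
; When BP_Player overlaps the box, it disables player input, plays a Level Sequence and waits for its duration.
; It then moves the player to a hardcoded world location, restores input, calls InteractWith on the NPC and destroys itself.
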(event `self.Box.OnComponentBeginOverlap`
  (params (OverlappedComponent :type "PrimitiveComponent Object Reference") (OtherActor :type "Actor Object Reference") (OtherComp :type "PrimitiveComponent Object Reference") (OtherBodyIndex :type Integer) (bFromSweep :type Boolean) (SweepResult :type "HitResult Structure (by ref)"))
  (bind _returnvalue (`GameplayStatics.GetPlayerCharacter` 0))
  (bind _returnvalue_2 (`GameplayStatics.GetPlayerController` 0))
  (cast `/Game/Player/BluePrints/BP_Player` OtherActor)
  (`self.DisableInput` _returnvalue _returnvalue_2)
  (bind (_outactor _returnvalue_3) (`LevelSequencePlayer.CreateLevelSequencePlayer` (`self.LevelSequence`)))
  (`MovieSceneSequencePlayer.Play` _returnvalue_3)
  (`KismetSystemLibrary.Delay` (`TimeManagementBlueprintLibrary.Conv_QualifiedFrameTimeToSeconds` (`MovieSceneSequencePlayer.GetDuration` _returnvalue_3)))
  (`self.K2_SetActorLocation` (`GameplayStatics.GetPlayerCharacter` 0) (9998.0 -7920.0 4333.0) false false)
  (`self.EnableInput` _returnvalue _returnvalue_2)
  (`/Game/GameSystems/BPI_Interaction.InteractWith` (`self.NPC`))
  (`self.K2_DestroyActor`))

(fn `UserConstructionScript`)